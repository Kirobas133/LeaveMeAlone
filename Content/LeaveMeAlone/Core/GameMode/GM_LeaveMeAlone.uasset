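; GM_LeaveMeAlone is the game mode that runs the match countdown and ends the game when time runs out.
; On BeginPlay it starts a looping one-second timer that decrements GameTime.
; At zero it clears the timer, pauses the game and shows the WBP_TimeOut widget with UI-only input and a visible mouse cursor.
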(event `self.ReceiveBeginPlay`
  (bind _returnvalue (`KismetSystemLibrary.K2_SetTimerDelegate` (delegate `CustomEvent`) 1.0 true))
  (bind _output_get (set `self.GameTimer` _returnvalue)))

(event `CustomEvent`
  (bind _returnvalue (`GameplayStatics.GetPlayerController` 0))
  (bind _output_get (set `self.Game Time` (- (`self.Game Time`) 1)))
  (if (== _output_get 0)
    (`KismetSystemLibrary.K2_ClearAndInvalidateTimerHandle` (stale `self.ReceiveBeginPlay` _output_get))
    (`GameplayStatics.SetGamePaused` true)
    (bind _returnvalue_2 (`|CreateWidget` "/Game/LeaveMeAlone/Widgets/UI/WBP_TimeOut.WBP_TimeOut_C"))
    (bind _output_get_2 (set `self.Time Out UI` _returnvalue_2))
    (`UserWidget.AddToViewport` _output_get_2 0)
    (`WidgetBlueprintLibrary.SetInputMode_UIOnlyEx` _returnvalue _output_get_2)
    (set `PlayerController.bShowMouseCursor` true _returnvalue)))

(fn `UserConstructionScript`)